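; Titan character Blueprint: an AI-driven character that runs a behavior tree and can be assigned to a building.
; Assign writes the target building and its reached/changed flags to the blackboard, and GetAssignedBuilding reads it back.
; Flag-controlled timelines loop a capsule mesh hop and a jump sound until StopInteractions clears them and resets the color to white.
; Color changes create a dynamic material instance on the capsule mesh.
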(event `self.ReceiveBeginPlay`
  (`AIController.RunBehaviorTree` (`AIBlueprintHelperLibrary.GetAIController` self) "/Game/AI/TinanCharacter_BT.TinanCharacter_BT"))

(event `/Game/Blueprints/CharacterInteractions.ChangeColor`
  (params (Color :type "Color Structure"))
  (bind _returnvalue (`PrimitiveComponent.CreateDynamicMaterialInstance` (`self.CapsuleMesh`) 0 "/Game/Resources/Materials/CharacterMaterial.CharacterMaterial" "None"))
  (`MaterialInstanceDynamic.SetVectorParameterValue` _returnvalue "Color" (`KismetMathLibrary.Conv_ColorToLinearColor` Color)))

(event `/Game/Blueprints/CharacterInteractions.StartJumping`
  (set `self.IsJumping` true)
  (if (`self.IsJumping`) :!label _label
    (bind (_direction _zoffset) (`Timeline|Timeline` :!via `PlayFromStart`)
      (:`Update`
        (`SceneComponent.K2_SetRelativeLocation` (`self.CapsuleMesh`) (`KismetMathLibrary.MakeVector` 0.0 0.0 _zoffset) false false))
      (:`Finished`
        (goto _label)))))

(event `/Game/Blueprints/CharacterInteractions.StartPlayingSound`
  (set `self.IsPlayingSound` true)
  (if (`self.IsPlayingSound`) :!label _label_2
    (`Timeline|Timeline_0` :!via `PlayFromStart`
      (:`Finished`
        (goto _label_2))
      (:`SoundTrack`
        (`GameplayStatics.PlaySound2D` "/Game/Resources/jump_sound.jump_sound" 1.0 1.0 0.0 null null)))))

(event `/Game/Blueprints/CharacterInteractions.StopInteractions`
  (set `self.IsJumping` false)
  (set `self.IsPlayingSound` false)
  (`self.ModifyColor` (make `Color` 255 255 255 255)))

(fn `Assign`
  (params (Building :type "/Game/Blueprints/BuildingBase Object Reference"))
  (`BlackboardComponent.SetValueAsObject` (`AIBlueprintHelperLibrary.GetBlackboard` null) "Building" Building)
  (`BlackboardComponent.SetValueAsBool` (`AIBlueprintHelperLibrary.GetBlackboard` null) "IsBuildingReached" false)
  (`BlackboardComponent.SetValueAsBool` (`AIBlueprintHelperLibrary.GetBlackboard` null) "HasTargetBuildingChanged" true))

(fn `GetAssignedBuilding`
  (returns (Value :type "/Game/Blueprints/BuildingBase Object Reference"))
  (bind _asbuilding_base (cast `/Game/Blueprints/BuildingBase` (`BlackboardComponent.GetValueAsObject` (`AIBlueprintHelperLibrary.GetBlackboard` (`AIBlueprintHelperLibrary.GetAIController` self)) "Building"))
    (:`then`
      (return _asbuilding_base))
    (:`CastFailed`
      (return null))))

(fn `ModifyColor`
  (params (Color :type "Color Structure"))
  (bind _returnvalue (`PrimitiveComponent.CreateDynamicMaterialInstance` (`self.CapsuleMesh`) 0 "/Game/Resources/Materials/CharacterMaterial.CharacterMaterial" "None"))
  (`MaterialInstanceDynamic.SetVectorParameterValue` _returnvalue "Color" (`KismetMathLibrary.Conv_ColorToLinearColor` Color)))

(fn `UserConstructionScript`)