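; BuildingSelectionManager tracks the selected building and controls the visibility of building UI.
; On BeginPlay it finds every BuildingBase actor and binds to its selected and assigned-toggled events.
; Selecting a building hides the previous selection's UI, stores the new building and shows its UI.
; Any assignment toggle hides the UI of the currently selected building.
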(event `Building Assign Toggled`
  (params (Assigned :type Boolean))
  (`/Game/Blueprints/BuildingBase.SetUIVisible` (`self.SelectedBuilding`) false))

(event `self.ReceiveBeginPlay`
  (bind _outactors (`GameplayStatics.GetAllActorsOfClass` "/Game/Blueprints/BuildingBase.BuildingBase_C"))
  (for _array_element _outactors
    (add `/Game/Blueprints/BuildingBase.OnSelected` _array_element (delegate `BuildingSelected`))
    (add `/Game/Blueprints/BuildingBase.OnAssignedToggled` _array_element (delegate `Building Assign Toggled`))))

(event `BuildingSelected`
  (params (SelectedBuilding :type "/Game/Blueprints/BuildingBase Object Reference"))
  (`|ExecutionSequence`
    (:`then_0`
      (if (!= (`self.SelectedBuilding`) null)
        (`/Game/Blueprints/BuildingBase.SetUIVisible` (`self.SelectedBuilding`) false)))
    (:`then_1`
      (bind _output_get (set `self.SelectedBuilding` SelectedBuilding))
      (`/Game/Blueprints/BuildingBase.SetUIVisible` _output_get true))))

(fn `UserConstructionScript`)