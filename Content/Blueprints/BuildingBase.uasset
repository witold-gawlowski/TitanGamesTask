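; BuildingBase is a base building actor that can be clicked to select it and assigned to or unassigned from the TitanCharacter.
; On BeginPlay it caches the character, initializes the AssignWidget from its widget component and binds the button.
; Clicking broadcasts selection and refreshes the widget text; ToggleAssign flips assignment, which the character stores, and broadcasts the change.
; UI visibility and text have setter functions, while StartWork is an empty stub taking a worker.
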(event `Event ToggleAssign`
  (bind _value (`/Game/Blueprints/TitanCharacter.GetAssignedBuilding` (`self.MainCharacter`)))
  (if (== _value self)
    (`/Game/Blueprints/TitanCharacter.Assign` (`self.MainCharacter`) null)
    (`self.OnAssignedToggled` false)
    (else
      (`/Game/Blueprints/TitanCharacter.Assign` (`self.MainCharacter`) self)
      (`self.OnAssignedToggled` true))))

(event `self.ReceiveBeginPlay`
  (bind _asassign_widget (cast `/Game/Blueprints/AssignWidget` (`WidgetComponent.GetUserWidgetObject` (`self.Widget`))))
  (bind _output_get (set `self.AssignWidget` _asassign_widget))
  ;[1 1 1] Bind Events
  (add `/Game/Blueprints/AssignWidget.ButtonClicked` _output_get (`|CreateDelegate` :!event `Event ToggleAssign`))
  ;[1 1 1] Set Main Character
  (bind _returnvalue (`GameplayStatics.GetActorOfClass` "/Game/Blueprints/TitanCharacter.TitanCharacter_C"))
  (set `self.MainCharacter` _returnvalue)
  (`/Game/Blueprints/AssignWidget.Iniitialize` (`self.AssignWidget`) self))

(event `self.ReceiveActorOnClicked`
  (params (ButtonPressed :type "Key Structure"))
  (`self.OnSelected` self)
  (bind _value (`/Game/Blueprints/TitanCharacter.GetAssignedBuilding` (`self.MainCharacter`)))
  (`/Game/Blueprints/AssignWidget.SetTextAssigned` (`self.AssignWidget`) (== _value self)))

(fn `SetUIText`
  (params (Assigned :type Boolean))
  (`/Game/Blueprints/AssignWidget.SetTextAssigned` (`self.AssignWidget`) Assigned))

(fn `SetUIVisible`
  (params (Value :type Boolean))
  (`/Game/Blueprints/AssignWidget.SetVisible` (`self.AssignWidget`) Value))

(fn `StartWork`
  (params (Worker :type "/Game/Blueprints/TitanCharacter Object Reference")))

(fn `UserConstructionScript`)